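; BP_AIEnemy is an AI enemy that chases the player once it spots a pawn.
; PawnSensing sets IsSeeingPlayer on seeing any pawn and calls FollowPlayer, which issues an AI MoveTo toward the first player character.
; Tick stops movement while the flag is false.
; The flag is only cleared in a branch where it is already false, so it stays set after the first sighting.
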(event OnSeePawn(PawnSensing)
  (params (Pawn :type Pawn%20Object%20Reference))
  ;[0.15 0.15 0.15 0.5] Follow player
  (Variables|Default|SetIsSeeingPlayer true)
  (CallFunction|FollowPlayer))

(event Custom|FollowPlayer
  ;[0.15 0.15 0.15 0.5] Follow player
  (if (Variables|Default|GetIsSeeingPlayer)
    (AI|AIMoveTo self "0, 0, 0" (Game|GetPlayerCharacter 0) 5e+01 false)
    (else
      (Variables|Default|SetIsSeeingPlayer false))))

(event EventBeginPlay)

(event Collision|EventActorBeginOverlap
  (params (OtherActor :type Actor%20Object%20Reference)))

(event EventTick
  (params (DeltaSeconds :type Float%20%28single-precision%29))
  ;[0.15 0.15 0.15 0.5] Follow player
  (if (not (Variables|Default|GetIsSeeingPlayer))
    (Components|Movement|StopMovementImmediately (Variables|Character|GetCharacterMovement))))

(fn ConstructionScript)